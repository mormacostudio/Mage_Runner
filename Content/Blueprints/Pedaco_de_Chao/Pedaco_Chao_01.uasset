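; Floor segment for an endless runner that extends the track and removes itself once the player passes.
; Construction randomly picks between a possible obstacle at the center point and coins rolled independently at nine spawn points, added as child actor components.
; When PersonagemPrincipal overlaps the spawn collision, it asks RunnerGameMod to add the next segment, then destroys itself after a short delay.
; GetPontoEncaixe exposes the world transform of the attachment point for chaining segments.
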(event `self.ReceiveTick`
  (params (DeltaSeconds :type "Float (single-precision)")))

(event `self.Spawn_PedacoChao_COL.OnComponentBeginOverlap`
  (params (OverlappedComponent :type "PrimitiveComponent Object Reference") (OtherActor :type "Actor Object Reference") (OtherComp :type "PrimitiveComponent Object Reference") (OtherBodyIndex :type Integer) (bFromSweep :type Boolean) (SweepResult :type "HitResult Structure (by ref)"))
  ;[1 1 1] Cria o caminho e Destroi o caminho ultrapassado a cada 2 segundos
  (cast `/Game/Blueprints/Character/PersonagemPrincipal` OtherActor)
  (bind _asrunner_game_mod (cast `/Game/Blueprints/RunnerGameMod` (`GameplayStatics.GetGameMode`)))
  (`/Game/Blueprints/RunnerGameMod.AddPedacoChao` _asrunner_game_mod)
  (`KismetSystemLibrary.Delay` 2.0)
  (`self.K2_DestroyActor`))

(fn `CriaMoedas`
  (bind _output_get (set `self.Pontos_Moedas_VAR` (`|MakeArray` (`SceneComponent.GetRelativeTransform` (`self.Spawn_02`)) (`SceneComponent.GetRelativeTransform` (`self.Spawn_03`)) (`SceneComponent.GetRelativeTransform` (`self.Spawn_04`)) (`SceneComponent.GetRelativeTransform` (`self.Spawn_05`)) (`SceneComponent.GetRelativeTransform` (`self.Sapwn_01`)) (`SceneComponent.GetRelativeTransform` (`self.Spawn_07`)) (`SceneComponent.GetRelativeTransform` (`self.Spawn_08`)) (`SceneComponent.GetRelativeTransform` (`self.Spawn_09`)) (`SceneComponent.GetRelativeTransform` (`self.Spawn_06`)))))
  (bind _output_get_2 (set `self.Should_Happen_VAR` (`|MakeArray` (`KismetMathLibrary.RandomBoolWithWeight` 0.5) (`KismetMathLibrary.RandomBoolWithWeight` 0.5) (`KismetMathLibrary.RandomBoolWithWeight` 0.5) (`KismetMathLibrary.RandomBoolWithWeight` 0.5) (`KismetMathLibrary.RandomBoolWithWeight` 0.5) (`KismetMathLibrary.RandomBoolWithWeight` 0.5) (`KismetMathLibrary.RandomBoolWithWeight` 0.5) (`KismetMathLibrary.RandomBoolWithWeight` 0.5) (`KismetMathLibrary.RandomBoolWithWeight` 0.5))))
  (if (`|GetArrayItem` _output_get_2)
    (`AddComponent|NODE_AddChildActorComponent-2` :`RelativeTransform` (`|GetArrayItem` _output_get)))
  (if (`|GetArrayItem` _output_get_2 1)
    (`AddComponent|NODE_AddChildActorComponent-3` :`RelativeTransform` (`|GetArrayItem` _output_get 1)))
  (if (`|GetArrayItem` _output_get_2 2)
    (`AddComponent|NODE_AddChildActorComponent-4` :`RelativeTransform` (`|GetArrayItem` _output_get 2)))
  (if (`|GetArrayItem` _output_get_2 3)
    (`AddComponent|NODE_AddChildActorComponent-5` :`RelativeTransform` (`|GetArrayItem` _output_get 3)))
  (if (`|GetArrayItem` _output_get_2 4)
    (`AddComponent|NODE_AddChildActorComponent-6` :`RelativeTransform` (`|GetArrayItem` _output_get 4)))
  (if (`|GetArrayItem` _output_get_2 5)
    (`AddComponent|NODE_AddChildActorComponent-7` :`RelativeTransform` (`|GetArrayItem` _output_get 5)))
  (if (`|GetArrayItem` _output_get_2 6)
    (`AddComponent|NODE_AddChildActorComponent-8` :`RelativeTransform` (`|GetArrayItem` _output_get 6)))
  (if (`|GetArrayItem` _output_get_2 7)
    (`AddComponent|NODE_AddChildActorComponent-9` :`RelativeTransform` (`|GetArrayItem` _output_get 7)))
  (if (`|GetArrayItem` _output_get_2 8)
    (`AddComponent|NODE_AddChildActorComponent-10` :`RelativeTransform` (`|GetArrayItem` _output_get 8))))

(fn `CriaObstaculo`
  (bind _pontosobstaculos (`self.PontosObstaculos`))
  (if (`KismetMathLibrary.RandomBoolWithWeight` 0.5)
    (`AddComponent|NODE_AddChildActorComponent-0` :`RelativeTransform` (`|GetArrayItem` _pontosobstaculos (`KismetMathLibrary.RandomIntegerInRange` 0 (`KismetArrayLibrary.Array_LastIndex` _pontosobstaculos))))))

(fn `GetPontoEncaixe`
  (returns (PontoEncaixe :type "Transform Structure"))
  ;[1 1 1] Retorna o Valor para quem Chamar a função
  (return (`SceneComponent.K2_GetComponentToWorld` (`self.PontoEncaixe`))))

(fn `SetPontoObstaculo`
  (set `self.PontosObstaculos` (`|MakeArray` (`SceneComponent.GetRelativeTransform` (`self.PontoObstaculoCentro`)))))

(fn `UserConstructionScript`
  (`self.SetPontoObstaculo`)
  (switch `int` (`KismetMathLibrary.RandomIntegerInRange` 0 1)
    (:`0`
      (`self.CriaObstaculo`))
    (:`1`
      (`self.CriaMoedas`))))