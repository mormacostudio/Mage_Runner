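; Runner game mode that builds the track by chaining spawned floor pieces, laying ten of them on BeginPlay.
; AddPedacoChao spawns a random class from PedacosDeChaoVAR at the stored attach point, then stores the new piece's GetPontoEncaixe as the next one.
; The player's MaxWalkSpeed gates variety: above a speed threshold the random pick covers five piece types, otherwise only the first three.
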(event `self.ReceiveBeginPlay`
  (for _ (range 10)
    (`self.AddPedacoChao`)))

(fn `AddPedacoChao`
  (bind _aspersonagem_principal (cast `/Game/Blueprints/Character/PersonagemPrincipal` (`GameplayStatics.GetPlayerPawn` 0)))
  (if (> (`KismetMathLibrary.FTrunc` (`CharacterMovementComponent.MaxWalkSpeed` (`Character.CharacterMovement` _aspersonagem_principal))) 620)
    ;[1 1 1] Spawn do Chão
    (bind _returnvalue (`|SpawnActorFromClass` (`|GetArrayItem` (`self.Pedacos_de_Chao_VAR`) (`KismetMathLibrary.RandomIntegerInRange` 0 4)) (`self.PróximoPontoEncaixe`) "Undefined" "OverrideRootScale" null null))
    (bind _aspedaco_chao_01 (cast `/Game/Blueprints/Pedaco_de_Chao/Pedaco_Chao_01` _returnvalue))
    (bind _pontoencaixe (`/Game/Blueprints/Pedaco_de_Chao/Pedaco_Chao_01.GetPontoEncaixe` _aspedaco_chao_01))
    (set `self.PróximoPontoEncaixe` _pontoencaixe)
    (else
      (bind _returnvalue_2 (`|SpawnActorFromClass` (`|GetArrayItem` (`self.Pedacos_de_Chao_VAR`) (`KismetMathLibrary.RandomIntegerInRange` 0 2)) (`self.PróximoPontoEncaixe`) "Undefined" "OverrideRootScale" null null))
      (bind _aspedaco_chao_01_2 (cast `/Game/Blueprints/Pedaco_de_Chao/Pedaco_Chao_01` _returnvalue_2))
      (bind _pontoencaixe_2 (`/Game/Blueprints/Pedaco_de_Chao/Pedaco_Chao_01.GetPontoEncaixe` _aspedaco_chao_01_2))
      (set `self.PróximoPontoEncaixe` _pontoencaixe_2))))

(fn `UserConstructionScript`)