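; Enemy character for a runner game that moves itself each tick and fires a projectile-style power from its hand.
; Movement input runs opposite the control-yaw forward vector, and a tick counter periodically raises max walk speed.
; The cached RunnerGameMod's first attack flag triggers a delayed, DoOnce-gated spawn of Power_Enemy_BP at the right-hand socket.
; While that flag is off, a delayed event resets the gate.
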(event `Spawn_Power`
  (`KismetSystemLibrary.Delay` 0.2)
  (`/Engine/EditorBlueprintResources/StandardMacros.DoOnce` false :!label _label
    (:`Completed`
      (`self.Is_Attack_FCT`))))

(event `self.ReceiveBeginPlay`
  (bind _asrunner_game_mod (cast `/Game/Blueprints/RunnerGameMod` (`GameplayStatics.GetGameMode`)))
  (set `self.Conection_GameMode_VAR` _asrunner_game_mod))

(event `Reset_Spawn_Power`
  (`KismetSystemLibrary.Delay` 0.5)
  (goto _label :!via `Reset`))

(event `self.ReceiveTick`
  (params (DeltaSeconds :type "Float (single-precision)"))
  (if (`|GetArrayItem` (`/Game/Blueprints/RunnerGameMod.Enemy_Attack_VAR` (`self.Conection_GameMode_VAR`)))
    (`self.Spawn_Power`)
    (else
      (`self.Reset_Spawn_Power`)))
  (`self.AddMovementInput` (`KismetMathLibrary.GetForwardVector` (`KismetMathLibrary.MakeRotator` 0.0 0.0 (.yaw (`self.GetControlRotation`)))) -1.0)
  (bind _output_get (set `self.Time_Enemy_VAR` (+ (`self.Time_Enemy_VAR`) 10)))
  (if (== _output_get 1000)
    (set `self.Time_Enemy_VAR` 0)
    (`self.Add_Enemy_Velocity`)))

(fn `Add_Enemy_Velocity`
  (set `CharacterMovementComponent.MaxWalkSpeed` (+ (`CharacterMovementComponent.MaxWalkSpeed` (`self.CharacterMovement`)) 5.0) (`self.CharacterMovement`)))

(fn `Is_Attack_FCT`
  (`/Engine/EditorBlueprintResources/StandardMacros.DoOnce` false
    (:`Completed`
      (`|SpawnActorFromClass` "/Game/Blueprints/Power_Enemy_BP.Power_Enemy_BP_C" (`KismetMathLibrary.Conv_VectorToTransform` (`SceneComponent.GetSocketLocation` (`self.Mesh`) "Hand_RIght_SKT")) "Undefined" "OverrideRootScale" null null))))

(fn `UserConstructionScript`)